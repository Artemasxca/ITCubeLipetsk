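; BP_door is an interactable double door that opens once when the player interacts with it.
; The OnInterected event from BPC_InteractableObject plays a Timeline that lerps the two static meshes 45 degrees in opposite directions.
; Each Timeline update also hides the interaction widget.
; When the Timeline finishes, the interactable component is destroyed, so the door cannot be used again.
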(event OnInterected(BPC_InteractableObject)
  ;[1 1 1] Открывание двери
  (if true
    (bind _newtrack_0 (Timeline|Timeline Play)
      (:Update
        (Utilities|FlowControl|Sequence
          (:then_0
            (Transformation|SetRelativeRotation (Variables|Default|GetStaticMesh) (Math|Rotator|Lerp(Rotator) "0, 0, 0" "0.000000,-45.000000,0.000000" _newtrack_0) false false))
          (:then_1
            (Transformation|SetRelativeRotation (Variables|Default|GetStaticMesh1) (Math|Rotator|Lerp(Rotator) "0.000000,180.000000,0.000000" "0.000000,225.000000,0.000000" _newtrack_0) false false)))
        (Default|ShowInteractionWidget (Variables|Collision|GetBPC_InteractableObject) false))
      (:Finished
        (if true
          (Components|DestroyComponent (Variables|Collision|GetBPC_InteractableObject)))))))

(event EventBeginPlay)

(event Collision|EventActorBeginOverlap
  (params (OtherActor :type Actor%20Object%20Reference)))

(event EventTick
  (params (DeltaSeconds :type Float%20%28single-precision%29)))

(fn ConstructionScript)